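; BP_Tank is a tank Blueprint that sets up its aiming component and handles camera look input.
; On BeginPlay it passes its barrel and turret to TankAiming.
; LookH yaws the Scene component, while LookV pitches the SpringArm within a clamped range, splitting horizontal and vertical rotation across two components.
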(event EventBeginPlay
  (Class|TankAimingComponent|Initialize (Variables|Default|GetTankAiming) (Variables|Default|GetTankBarrel) (Variables|Default|GetTankTurret)))

(event Input|AxisEvents|InputAxisLookV
  (params (AxisValue :type Float%20%28single-precision%29))
  (bind _springarm (Variables|Default|GetSpringArm))
  (bind _relativerotation (Variables|/Script/Engine.SceneComponent|GetRelativeRotation _springarm))
  (Transformation|SetRelativeRotation (Variables|Default|GetSpringArm) (Math|Rotator|MakeRotator (.roll _relativerotation) (Math|Float|Clamp(Float) (+ AxisValue (.pitch _relativerotation)) -4e+01 5.0) (.yaw _relativerotation)) false false))

(event Input|AxisEvents|InputAxisLookH
  (params (AxisValue :type Float%20%28single-precision%29))
  (Transformation|AddRelativeRotation (Variables|Default|GetScene) (Math|Rotator|MakeRotator 0.0 0.0 AxisValue) false false))

(fn ConstructionScript)