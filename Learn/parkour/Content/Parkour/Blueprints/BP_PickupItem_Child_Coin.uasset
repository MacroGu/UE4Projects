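; Coin pickup for the parkour game, a child of a pickup item Blueprint that adds to the coin count when grabbed.
; On BeginPlay it runs the parent logic and binds a handler to the inherited OnPickup dispatcher.
; The handler casts the game mode to ParkourGameMode, increments its coins by one and plays a score sound at the coin's location.
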(event Custom|PickupGrabbed
  (bind _asparkour_game_mode (Utilities|Casting|CastToParkourGameMode (Game|GetGameMode)))
  (Default|IncrementCoin _asparkour_game_mode 1)
  (Audio|PlaySoundatLocation "/Game/Parkour/Audio/SFX_Score_01.SFX_Score_01" (Transformation|GetActorLocation)))

(event EventBeginPlay
  (|CallParentFunction)
  (EventDispatchers|AssignOnPickup (delegate Custom|PickupGrabbed)))

(event Collision|EventActorBeginOverlap
  (params (OtherActor :type Actor%20Object%20Reference))
  (|CallParentFunction OtherActor) ; This node is disabled and will not be called.\nDrag off pins to build functionality.
)

(event EventTick
  (params (DeltaSeconds :type Float%20%28single-precision%29))
  (|CallParentFunction DeltaSeconds) ; This node is disabled and will not be called.\nDrag off pins to build functionality.
)

(fn ConstructionScript
  (|CallParentFunction))