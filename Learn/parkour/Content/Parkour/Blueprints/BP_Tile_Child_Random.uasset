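; Random parkour tile child that fills three component slots with floor, obstacles or empty classes and assigns coins to one slot.
; Its construction script rolls the layout, calls SpawnAllTileComponnet, then picks a coin slot independently of the layout and calls PlaceAllCoins.
; Weighted rolls favor all floor, then one non-floor slot, and rarely two, always keeping at least one floor.
; Each non-floor slot randomly becomes a blocker, wall or no class.
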(event EventBeginPlay
  (|CallParentFunction) ; This node is disabled and will not be called.\nDrag off pins to build functionality.
)

(event Collision|EventActorBeginOverlap
  (params (OtherActor :type Actor%20Object%20Reference))
  (|CallParentFunction OtherActor) ; This node is disabled and will not be called.\nDrag off pins to build functionality.
)

(event EventTick
  (params (DeltaSeconds :type Float%20%28single-precision%29))
  (|CallParentFunction DeltaSeconds) ; This node is disabled and will not be called.\nDrag off pins to build functionality.
)

(fn ConstructionScript
  (|CallParentFunction)
  (Utilities|FlowControl|Sequence
    (:then_0
      (|CreateTileComponentClasses))
    (:then_1
      (CallFunction|SpawnAllTileComponnet))
    (:then_2
      (|CreateCoins))))

(fn RandomTileComponentClassWithoutFloor
  (switch int (Math|Random|RandomInteger 3)
    (:0
      (LocalVariables|SetNewLocalVar_0 0))
    (:1
      (LocalVariables|SetNewLocalVar_0 "/Game/Parkour/Blueprints/BP_TileComponent_Child_Blocker.BP_TileComponent_Child_Blocker_C"))
    (:2
      (LocalVariables|SetNewLocalVar_0 "/Game/Parkour/Blueprints/BP_TileComponent_Child_Wall.BP_TileComponent_Child_Wall_C")))
  (return (LocalVariables|GetNewLocalVar_0)))