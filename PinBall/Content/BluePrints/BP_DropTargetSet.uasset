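; BP_DropTargetSet is a row of drop targets between two posts that spells a word and resets once every target is down.
; The construction script uppercases PostString and spawns one child BP_DropTarget per character, spaced evenly by the post distance and labeled with its letter.
; Each target's OnTargetDrop event is bound for counting drops.
; TargetDropProcess decrements the counter and, at zero, waits briefly, resets all targets and restores the count.
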(event Custom|TargetDropProcess
  (bind _droptargets (Variables|Default|GetDropTargets))
  (bind _result (Math|Integer|DecrementInt (Variables|Default|GetTargetCounter))
    (:%20%20
      (if (<= _result 0)
        (Utilities|FlowControl|Delay 1.0)
        (for _array_element _droptargets
          (Default|ResetDrop _array_element)
          (Variables|Default|SetTargetCounter (Utilities|Array|Length _droptargets)))))))

(event EventBeginPlay
  (|CallParentFunction))

(event Collision|EventActorBeginOverlap
  (params (OtherActor :type Actor%20Object%20Reference))
  (|CallParentFunction OtherActor))

(event EventTick
  (params (DeltaSeconds :type Float%20%28single-precision%29))
  (|CallParentFunction DeltaSeconds))

(fn ConstructionScript
  (bind _post1 (Variables|Default|GetPost1))
  (|CallParentFunction)
  (bind _output_get (Variables|Default|SetPostString (Class|KismetStringLibrary|ToUpper (Variables|Default|GetPostString))))
  (Variables|Default|SetTargetCounter (Utilities|Array|Length (Utilities|String|GetCharacterArrayfromString _output_get)))
  (for (_array_element _array_index) (Utilities|String|GetCharacterArrayfromString _output_get)
    (bind _returnvalue (AddComponent|AddChildActorComponent false (Math|Transform|MakeTransform (+ (* (Math|Vector|GetForwardVector _post1) (* (/ (Math|Vector|VectorLength (- (Variables|/Script/Engine.SceneComponent|GetRelativeLocation (Variables|Default|GetPost1)) (Variables|/Script/Engine.SceneComponent|GetRelativeLocation (Variables|Default|GetPost2)))) (Math|Conversions|ToFloat(Integer) (+ (Utilities|Array|Length (Utilities|String|GetCharacterArrayfromString _output_get)) 1))) (Math|Conversions|ToFloat(Integer) (+ _array_index 1)))) (* (Math|Vector|GetRightVector _post1) 3e+01)) (Transformation|GetWorldRotation _post1) "1,1,1")))
    (bind _asbp_drop_target (Utilities|Casting|CastToBP_DropTarget (Variables|/Script/Engine.ChildActorComponent|GetChildActor _returnvalue)))
    (Utilities|Array|Add (Variables|Default|GetDropTargets) _asbp_drop_target)
    (Rendering|Components|TextRender|SetText (Variables|/Game/BluePrints/BP_DropTarget.BP_DropTarget_C|GetDropText _asbp_drop_target) (Utilities|Text|ToText(String) _array_element))
    (EventDispatchers|BindEventtoOnTargetDrop _asbp_drop_target (EventDispatchers|CreateEvent :!event Custom|TargetDropProcess))))