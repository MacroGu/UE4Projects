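; Pinball game mode that keeps a ball in play, spawning one at BeginPlay and a replacement whenever it is destroyed.
; SpawnBall resets TiltCount from the class defaults, then spawns a BP_PinBall at the spawn location supplied by the first BP_Plunger found in the level.
; Each new ball's OnDestroyed event is bound back to SpawnBall, forming an endless respawn loop with no ball limit.
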(event Custom|SpawnBall
  (Variables|Default|SetTiltCount (Utilities|GetClassDefaults "PinBallGameMode_C"))
  (bind _outactors (Actor|GetAllActorsOfClass "/Game/BluePrints/BP_Plunger.BP_Plunger_C"))
  (bind _returnvalue (Game|SpawnActorfromClass "/Game/BluePrints/BP_PinBall.BP_PinBall_C" (Math|Transform|MakeTransform (Default|GetSpawnLocationWorld (Utilities|Array|Get(acopy) _outactors)) "0, 0, 0" "1,1,1") "Undefined" 0 0))
  (Game|BindEventtoOnDestroyed _returnvalue (delegate Custom|OnBallDestroyed)))

(event Custom|OnBallDestroyed
  (params (DestroyedActor :type Actor%20Object%20Reference))
  (CallFunction|SpawnBall))

(event EventBeginPlay
  (CallFunction|SpawnBall))

(event EventTick
  (params (DeltaSeconds :type Float%20%28single-precision%29)))

(fn ConstructionScript)