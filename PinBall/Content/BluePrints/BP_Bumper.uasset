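; Pinball bumper actor that kicks any BP_PinBall overlapping it away from its center.
; The overlap calls Bump, which replaces the ball's velocity with a fixed-speed push along the bumper-to-ball direction and spawns a sound and particle effect.
; A timeline then drives the bumper mesh's vertical offset, the base material's emissive glow and the point light intensity from one alpha curve.
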(event Custom|Bump
  (params (Ball :type BP%20Pin%20Ball%20Object%20Reference))
  (Physics|SetPhysicsLinearVelocity (Variables|/Game/BluePrints/BP_PinBall.BP_PinBall_C|GetBall Ball) (* (Math|Vector|GetUnitDirection(Vector) (Transformation|GetActorLocation) (Transformation|GetActorLocation Ball)) 2e+03) false "None")
  (Audio|SpawnSoundAttached "/Game/Assests/Sounds/Cue_Bumper.Cue_Bumper" (Variables|Default|GetBumperBase))
  (Effects|SpawnEmitteratLocation "/Game/Assests/Particles/P_Bumper.P_Bumper" (Transformation|GetWorldLocation (Variables|Default|GetBumperBase)))
  (bind _bumperalpha (Timeline|BumperTimeline PlayFromStart)
    (:Update
      (Transformation|SetRelativeLocation (Variables|Default|GetBumperBot) (Math|Vector|Lerp(Vector) "0, 0, 0" "0, 0,70.000000" _bumperalpha) false false)
      (Rendering|Material|SetScalarParameterValueonMaterials (Variables|Default|GetBumperBase) "Emissive" (Math|Float|Lerp 0.0 2e+01 _bumperalpha))
      (Rendering|Components|Light|SetIntensity (Variables|Default|GetPointLight) (Math|Float|Lerp 0.0 8e+03 _bumperalpha)))))

(event EventBeginPlay)

(event Collision|EventActorBeginOverlap
  (params (OtherActor :type Actor%20Object%20Reference))
  (bind _asbp_pin_ball (Utilities|Casting|CastToBP_PinBall OtherActor))
  (CallFunction|Bump _asbp_pin_ball))

(event EventTick
  (params (DeltaSeconds :type Float%20%28single-precision%29)))

(fn ConstructionScript)