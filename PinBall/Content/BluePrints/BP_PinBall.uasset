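; Pinball actor that drives its physics ball and its rolling sound every tick.
; Rolling cue volume and pitch scale with the actor's velocity, clamped to set ranges.
; The ball gets a frame-scaled velocity-change impulse along world X from Speed.
; A downward line trace finds the surface normal, and a second impulse, scaled by Stickness, presses the ball against that surface.
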(event EventBeginPlay)

(event EventTick
  (params (DeltaSeconds :type Float%20%28single-precision%29))
  (bind _returnvalue (Transformation|GetVelocity))
  (bind _returnvalue_2 (Transformation|GetActorLocation))
  (bind _pinball_rolling01_cue (Variables|Default|GetPinball_Rolling01_Cue))
  (bind _returnvalue_3 (Math|Vector|VectorLength _returnvalue))
  (bind _returnvalue_4 (/ _returnvalue_3 2e+03))
  (Utilities|FlowControl|Sequence
    (:then_0
      (Audio|Components|Audio|SetVolumeMultiplier _pinball_rolling01_cue (Math|Float|Clamp(Float) _returnvalue_4 0.0 1.2) :!class /Script/Engine.AudioComponent)
      (Audio|Components|Audio|SetPitchMultiplier _pinball_rolling01_cue (Math|Float|Clamp(Float) _returnvalue_4 0.9 1.1)))
    (:then_1
      (Physics|AddImpulse (Variables|Default|GetBall) (Math|Vector|MakeVector (* DeltaSeconds (Variables|Default|GetSpeed)) 0.0 0.0) "None" true)
      (bind _outhit (Collision|LineTraceByChannel _returnvalue_2 (- _returnvalue_2 "0, 0,500.000000") "TraceTypeQuery1" false 0 "None"))
      (Physics|AddImpulse (Variables|Default|GetBall) (* (* (* (.ImpactNormal (Collision|BreakHitResult _outhit)) -1.0) (Variables|Default|GetStickness)) DeltaSeconds) "None" true))))

(fn ConstructionScript)