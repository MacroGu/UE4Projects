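; Player controller for a pinball game that maps input actions to flippers, the plunger and table tilting.
; On BeginPlay it finds all flippers, sorting them into left and right arrays, and caches the first plunger it finds.
; Tilting applies a sideways velocity impulse to every ball while the game mode's TiltCount lasts, using up one tilt and playing a direction-matched camera shake.
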(event Custom|FindAllFliper
  (bind _outactors (Actor|GetAllActorsOfClass "/Game/BluePrints/BP_Fliper.BP_Fliper_C"))
  (for _array_element _outactors
    (bind _asbp_fliper (Utilities|Casting|CastToBP_Fliper _array_element))
    (switch Utilities|FlowControl|Switch|SwitchonE_Direction (Variables|/Game/BluePrints/BP_Fliper.BP_Fliper_C|GetFliperType _asbp_fliper)
      (:NewEnumerator0
        (Utilities|Array|Add (Variables|Default|GetLeftFlipers) _asbp_fliper))
      (:NewEnumerator1
        (Utilities|Array|Add (Variables|Default|GetRightFlipers) _asbp_fliper)))))

(event Custom|FindPlunger
  (bind _outactors (Actor|GetAllActorsOfClass "/Game/BluePrints/BP_Plunger.BP_Plunger_C"))
  (Variables|Default|SetPlunger (Utilities|Array|Get(acopy) _outactors)))

(event EventBeginPlay
  (CallFunction|FindAllFliper)
  (CallFunction|FindPlunger))

(event EventTick
  (params (DeltaSeconds :type Float%20%28single-precision%29)))

(event Input|ActionEvents|InputActionLeftFlip
  (params (Key :type Key%20Structure))
  (bind _leftflipers (Variables|Default|GetLeftFlipers))
  (:Pressed
    (for _array_element _leftflipers
      (Default|FliperUp _array_element)))
  (:Released
    (for _array_element_2 _leftflipers
      (Default|FliperDown _array_element_2))))

(event Input|ActionEvents|InputActionTiltLeft
  (params (Key :type Key%20Structure))
  (:Pressed
    (CallFunction|Tilt "NewEnumerator0")))

(event Input|ActionEvents|InputActionRightFlip
  (params (Key :type Key%20Structure))
  (bind _rightflipers (Variables|Default|GetRightFlipers))
  (:Pressed
    (for _array_element _rightflipers
      (Default|FliperUp _array_element)))
  (:Released
    (for _array_element_2 _rightflipers
      (Default|FliperDown _array_element_2))))

(event Input|ActionEvents|InputActionTiltRight
  (params (Key :type Key%20Structure))
  (:Pressed
    (CallFunction|Tilt "NewEnumerator1")))

(event Input|ActionEvents|InputActionCharge
  (params (Key :type Key%20Structure))
  (bind _plunger (Variables|Default|GetPlunger))
  (:Pressed
    (Default|Charge _plunger))
  (:Released
    (Default|Release _plunger)))

(fn ConstructionScript)

(fn Tilt
  (params (Direction :type E_Direction%20Enum :default "NewEnumerator0"))
  (bind _returnvalue (Game|GetPlayerCameraManager 0))
  (bind _returnvalue_2 (Game|GetGameMode))
  (bind _returnvalue_3 (Camera|GetCameraRotation _returnvalue))
  (bind _aspin_ball_game_mode (Utilities|Casting|CastToPinBallGameMode _returnvalue_2))
  (bind _tiltcount (Variables|/Game/BluePrints/PinBallGameMode.PinBallGameMode_C|GetTiltCount _aspin_ball_game_mode))
  (if (>= _tiltcount 1)
    (bind _outactors (Actor|GetAllActorsOfClass "/Game/BluePrints/BP_PinBall.BP_PinBall_C"))
    (if (>= (Utilities|Array|Length _outactors) 1)
      (for _array_element _outactors
        (Physics|AddImpulse (Variables|/Game/BluePrints/BP_PinBall.BP_PinBall_C|GetBall _array_element) (Utilities|Select :Index Direction :NewEnumerator0 "0,-500.000000, 0" :NewEnumerator1 "0,500.000000, 0") "None" true))
      (Math|Integer|DecrementInt _tiltcount
        (:%20%20
          (Class|PlayerController|ClientPlayCameraShake "/Game/BluePrints/PinBallCamShake.PinBallCamShake_C" 1.0 "UserDefined" (Utilities|Select :Index Direction :NewEnumerator0 _returnvalue_3 :NewEnumerator1 (Math|Rotator|CombineRotators _returnvalue_3 "0,180.000000, 0"))))))))