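; Pinball flipper actor that serves as either the left or right flipper, chosen by FliperType.
; The construction script sets the rest and raised rotations per side, applies the rest rotation and mirrors the mesh on X for the right side.
; FliperUp plays a side-specific sound and uses MoveComponentTo to swing to the raised rotation, while FliperDown returns it to rest.
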(event Custom|FliperDown
  (Components|MoveComponentTo (Variables|Default|GetFliper) "0, 0, 0" (Variables|Default|GetStartRotation) false false 0.2 false))

(event Custom|FliperUp
  (Audio|SpawnSoundAttached (Utilities|Select :Index (Variables|Default|GetFliperType) :NewEnumerator0 "/Game/Assests/Sounds/Pinball_FlipperLeft_Cue.Pinball_FlipperLeft_Cue" :NewEnumerator1 "/Game/Assests/Sounds/Pinball_FlipperRight_Cue.Pinball_FlipperRight_Cue") (Variables|Default|GetFliper))
  (Components|MoveComponentTo (Variables|Default|GetFliper) "0, 0, 0" (Variables|Default|GetEndRotation) false false 0.2 false))

(event EventBeginPlay)

(event Collision|EventActorBeginOverlap
  (params (OtherActor :type Actor%20Object%20Reference)))

(event EventTick
  (params (DeltaSeconds :type Float%20%28single-precision%29)))

(fn ConstructionScript
  (Variables|Default|SetStartRotation (Utilities|Select :Index (Variables|Default|GetFliperType) :NewEnumerator0 "0,-70.000000, 0" :NewEnumerator1 "0,-110.000000, 0"))
  (Variables|Default|SetEndRotation (Utilities|Select :Index (Variables|Default|GetFliperType) :NewEnumerator0 "0,-120.000000, 0" :NewEnumerator1 "0,-60.000000, 0"))
  (Transformation|SetRelativeRotation (Variables|Default|GetFliper) (Variables|Default|GetStartRotation) false false)
  (switch Utilities|FlowControl|Switch|SwitchonE_Direction (Variables|Default|GetFliperType)
    (:NewEnumerator1
      (Transformation|SetRelativeScale3D (Variables|Default|GetFliper) "-1.000000,1.000000,1.000000"))))