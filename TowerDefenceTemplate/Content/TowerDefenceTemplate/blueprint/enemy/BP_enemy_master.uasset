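; BP_enemy_master is an enemy actor for a tower defence template, with health and armor.
; On BeginPlay it uses AI MoveTo to head for the first actor returned by a class search.
; Any damage is reduced by armor with a small minimum, subtracted from health and the remainder printed.
; The actor is destroyed only when health equals exactly zero, so overshooting below zero leaves it alive.
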(event EventBeginPlay
  (bind _outactors (Actor|GetAllActorsOfClass 0))
  (AI|AIMoveTo self "0, 0, 0" (Utilities|Array|Get(acopy) _outactors) 1.2e+02 false))

(event Game|Damage|EventAnyDamage
  (params (Damage :type Float%20%28single-precision%29) (DamageType :type Damage%20Type%20Object%20Reference) (InstigatedBy :type Controller%20Object%20Reference) (DamageCauser :type Actor%20Object%20Reference))
  (Development|PrintString (Utilities|String|ToString(Float) (- (Variables|attribute|Getenemy_health) (Math|Float|Clamp(Float) (- Damage (Variables|attribute|Getenemy_armor)) 0.1 999.0))))
  (bind _output_get (Variables|attribute|Setenemy_health (- (Variables|attribute|Getenemy_health) (Math|Float|Clamp(Float) (- Damage (Variables|attribute|Getenemy_armor)) 0.1 999.0))))
  (if (== _output_get 0.0)
    (Actor|DestroyActor)))

(fn ConstructionScript)