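; Master tower Blueprint for a tower defence game that finds enemies in range and fires weapon actors at them.
; A delayed search loop sphere-traces around the tower and targets the enemy nearest BP_base, using a remembered distance that is never reset here.
; Attacks optionally yaw the tower toward its target and play a fire montage, whose notify spawns the weapon at WeaponArrow.
; Attacks repeat until the target becomes invalid, then searching resumes.
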(event Custom|search_enemy
  (bind _returnvalue (Transformation|GetActorLocation))
  (Utilities|FlowControl|Delay 0.5)
  (bind (_outhits _returnvalue_2) (Collision|MultiSphereTraceForObjects _returnvalue _returnvalue (Variables|attribute|GetattachRange) (Utilities|Array|MakeArray "ObjectTypeQuery7") false 0 "ForDuration"))
  (if _returnvalue_2
    (Utilities|Array|Clear (Variables|gaming|GetsearchEnemyArray))
    (for _array_element _outhits
      (bind _asbp_enemy_master (Utilities|Casting|CastToBP_enemy_master (.HitActor (Collision|BreakHitResult _array_element))))
      (Utilities|Array|Add (Variables|gaming|GetsearchEnemyArray) _asbp_enemy_master))
    (if (>= (Utilities|Array|Length (Variables|gaming|GetsearchEnemyArray)) 1)
      (bind _hasenemy_ (CallFunction|FUCEnemyfromBaseDistance))
      (if _hasenemy_
        (CallFunction|Attack)
        (else
          (CallFunction|SearchEnemy :!label _label)))
      (else
        (goto _label)))
    (else
      (CallFunction|SearchEnemy))))

(event Custom|Attack
  (if (Variables|attribute|GetisAttackNoTurnBody)
    _
    (else
      (Transformation|SetActorRotation (Math|Rotator|MakeRotator 0.0 0.0 (.yaw (Math|Rotator|FindLookatRotation (Transformation|GetActorLocation) (Transformation|GetActorLocation (Variables|gaming|GetenemyToAttack))))))))
  (Animation|Montage|PlayMontage (Variables|Default|GettowerMesh) (Variables|reference|Getref_montage) 1.0 0.0 "fire"
    (:then
      (Variables|gaming|SetisAttack? true))
    (:OnCompleted
      (Utilities|FlowControl|Delay (Variables|attribute|GetattackTime))
      (Utilities|IsValid (Variables|gaming|GetenemyToAttack)
        (:Is%20Valid
          (CallFunction|Attack))
        (:Is%20Not%20Valid
          (Variables|gaming|SetisAttack? false)
          (CallFunction|SearchEnemy))))
    (:OnNotifyBegin
      (bind _returnvalue (Game|SpawnActorfromClass (Variables|reference|Getref_weaponClass) (Transformation|GetWorldTransform (Variables|Default|GetweaponArrow)) "Undefined" 0 0))
      (Utilities|Casting|CastToBP_weapon_Master _returnvalue))))

(event EventBeginPlay
  (bind _outactors (Actor|GetAllActorsOfClass "/Game/TowerDefenceTemplate/blueprint/aline/BP_base.BP_base_C"))
  (Variables|gaming|SetAlineBase (Utilities|Array|Get(acopy) _outactors))
  (CallFunction|SearchEnemy)
  (Utilities|FlowControl|Delay 0.58))

(event Collision|EventActorBeginOverlap
  (params (OtherActor :type Actor%20Object%20Reference)))

(event EventTick
  (params (DeltaSeconds :type Float%20%28single-precision%29)))

(event Game|Damage|EventAnyDamage
  (params (Damage :type Float%20%28single-precision%29) (DamageType :type Damage%20Type%20Object%20Reference) (InstigatedBy :type Controller%20Object%20Reference) (DamageCauser :type Actor%20Object%20Reference))
  (Development|PrintString (Utilities|String|ToString(Float) Damage)))

(fn ConstructionScript)

(fn FUCEnemyfromBaseDistance
  (for _array_element (Variables|gaming|GetsearchEnemyArray)
    (if (<= (Math|Vector|VectorLength (- (Transformation|GetActorLocation (Variables|gaming|GetAlineBase)) (Transformation|GetActorLocation _array_element))) (LocalVariables|GetenemyDistanceRemeber))
      (LocalVariables|SetenemyDistanceRemeber (Math|Vector|VectorLength (- (Transformation|GetActorLocation (Variables|gaming|GetAlineBase)) (Transformation|GetActorLocation _array_element))))
      (Variables|gaming|SetenemyToAttack _array_element)))
  (return (Utilities|IsValid (Variables|gaming|GetenemyToAttack))))